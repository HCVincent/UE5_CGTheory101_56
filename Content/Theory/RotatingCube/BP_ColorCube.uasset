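; BP_ColorCube is an actor that shows a vertex-colored cube spinning in yaw.
; The construction script builds a procedural mesh from the Vertices variable, hardcoded triangle indices and eight per-vertex colors, then applies M_VertexColorCube.
; Tick adds local yaw rotation scaled by RotationSpeed and delta time, keeping the spin frame-rate independent.
; An unconnected second mesh setup in the construction script never runs.
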(event EventBeginPlay)

(event Collision|EventActorBeginOverlap
  (params (OtherActor :type Actor%20Object%20Reference)))

(event EventTick
  (params (DeltaSeconds :type Float%20%28single-precision%29))
  (Transformation|AddActorLocalRotation (Math|Rotator|MakeRotator 0.0 0.0 (* DeltaSeconds (Variables|Default|GetRotationSpeed))) false false))

(fn ConstructionScript
  (bind _proceduralmesh (Variables|Default|GetProceduralMesh))
  (Class|ProceduralMeshComponent|CreateMeshSectionLinearColor _proceduralmesh 0 (Variables|Default|GetVertices) (Utilities|Array|MakeArray 0 2 1 0 3 2 5 6 4 4 6 7 4 1 5 4 0 1 3 6 2 3 7 6 1 6 5 1 2 6 4 3 0 4 7 3) 0 0 0 0 0 (Utilities|Array|MakeArray "(R=1.000000,G=1.000000,B=1.000000,A=1.000000)" "" "(R=1.000000,G=0.000000,B=0.000000,A=1.000000)" "(R=0.000000,G=1.000000,B=0.000000,A=1.000000)" "(R=0.000000,G=0.000000,B=1.000000,A=1.000000)" "(R=1.000000,G=1.000000,B=0.000000,A=1.000000)" "(R=0.000000,G=1.000000,B=1.000000,A=1.000000)" "(R=1.000000,G=0.000000,B=1.000000,A=1.000000)") 0 false false)
  (Rendering|Material|SetMaterial _proceduralmesh 0 "/Game/Theory/RotatingCube/M_VertexColorCube.M_VertexColorCube"))